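; Physic_Door is a door Blueprint that plays wooden open and close sounds as its SMDoor component rotates.
; Each Tick compares the door's relative rotation to zero with a small tolerance to decide whether it is closed.
; An Opened flag latches the state, so each sound fires once per transition at the actor's location.
; The graph only reacts to rotation and contains no logic that moves the door.
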(event EventBeginPlay)

(event EventActorBeginOverlap
  (params (OtherActor :type Actor%20Object%20Reference)))

(event EventTick
  (params (DeltaSeconds :type Float%20%28single-precision%29))
  (bind _returnvalue (Transformation|GetActorLocation))
  (if (Math|Rotator|Equal(Rotator) (Variables|/Script/Engine.SceneComponent|GetRelativeRotation (Variables|Default|GetSM_Door)) "0, 0, 0" 5.0)
    (if (Variables|Default|GetOpened)
      (Audio|PlaySoundatLocation "/Game/SoundFX/wooden-door-close.wooden-door-close" _returnvalue)
      (Variables|Default|SetOpened false))
    (elif (not (Variables|Default|GetOpened))
      (Audio|SpawnSoundatLocation "/Game/SoundFX/wooden-door-open.wooden-door-open" _returnvalue)
      (Variables|Default|SetOpened true))))

(fn ConstructionScript)