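; Battery pickup actor that adds to the player character's BatteryCapacity when collected.
; On any actor overlap, it destroys itself if player 0 is below MaxBatteryCapacity, otherwise it prints a can't-carry message.
; The increment and debug print of the new count run in the Destroyed event, so destruction by other means also awards a battery.
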(event EventBeginPlay)

(event EventActorBeginOverlap
  (params (OtherActor :type Actor%20Object%20Reference)))

(event EventTick
  (params (DeltaSeconds :type Float%20%28single-precision%29)))

(event Collision|EventActorBeginOverlap
  (params (OtherActor :type Actor%20Object%20Reference))
  (bind _asplayer_character (Utilities|Casting|CastToPlayerCharacter (Game|GetPlayerCharacter 0)))
  (if (< (Variables|/Game/ThirdPersonBP/Blueprints/PlayerCharacter.PlayerCharacter_C|GetBattery%20Capacity _asplayer_character) (Variables|/Game/ThirdPersonBP/Blueprints/PlayerCharacter.PlayerCharacter_C|GetMax%20Battery%20Capacity _asplayer_character))
    (Actor|DestroyActor)
    (else
      (Development|PrintString "Can't carry any more battery" true true "(R=1.000000,G=0.000000,B=0.898843,A=1.000000)"))))

(event EventDestroyed
  (bind _asplayer_character (Utilities|Casting|CastToPlayerCharacter (Game|GetPlayerCharacter 0)))
  (Variables|/Game/ThirdPersonBP/Blueprints/PlayerCharacter.PlayerCharacter_C|SetBattery%20Capacity _asplayer_character (+ (Variables|/Game/ThirdPersonBP/Blueprints/PlayerCharacter.PlayerCharacter_C|GetBattery%20Capacity _asplayer_character) 1))
  (Development|PrintString (Utilities|String|ToString(Integer) (Variables|/Game/ThirdPersonBP/Blueprints/PlayerCharacter.PlayerCharacter_C|GetBattery%20Capacity _asplayer_character)) true true "(R=0.000000,G=1.000000,B=0.269892,A=1.000000)"))

(fn ConstructionScript)